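; VR player pawn with axis-driven movement and left-hand pickup of physics objects.
; Movement sets actor location without sweep along camera forward and right vectors, and BeginPlay uses Stage tracking origin when a headset is enabled.
; Left trigger or E line-traces from the left motion controller, disables physics on the hit component and attaches its actor to the controller.
; Release detaches it and restores physics.
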(event `InputAxis|MoveForward`
  (params (AxisValue :type "Float (single-precision)"))
  ;[1 1 1] Player_movement
  (`self.K2_SetActorLocation` (`self.Add Movement` AxisValue (`SceneComponent.GetForwardVector` (`self.Camera`)))))

(event `self.ReceiveBeginPlay`
  ;[1 1 1] Init
  (if (`HeadMountedDisplayFunctionLibrary.IsHeadMountedDisplayEnabled`)
    (`HeadMountedDisplayFunctionLibrary.SetTrackingOrigin` "Stage")))

(event `InputAxis|MoveRight`
  (params (AxisValue :type "Float (single-precision)"))
  ;[1 1 1] Player_movement
  (`self.K2_SetActorLocation` (`self.Add Movement` AxisValue (`SceneComponent.GetRightVector` (`self.Camera`)))))

(event `InputAction|Input_TriggerLeft`
  (params (Key :type "Key Structure"))
  ;[1 1 1] Holding and Droping of items
  (:`Pressed`
    (if (not (`self.Is Holding Object`)) :!label _label
      (`self.PickUpObject`)))
  (:`Released`
    (`self.DropObject` :!label _label_2)))

(event `Key|E`
  (params (Key :type "Key Structure"))
  ;[1 1 1] Holding and Droping of items
  (:`Pressed`
    (goto _label))
  (:`Released`
    (goto _label_2)))

(event `PickUpObject`
  (bind _motioncontrollerlefft (`self.MotionControllerLefft`))
  (bind _hit_component (`self.Hit Component`))
  (bind _returnvalue (`SceneComponent.K2_GetComponentLocation` _motioncontrollerlefft))
  ;[0.5086 0.5251 1] PickUp Object
  (bind (_outhit _returnvalue_2) (`KismetSystemLibrary.LineTraceSingleForObjects` :`Start` _returnvalue :`End` (+ _returnvalue (* (`SceneComponent.GetForwardVector` _motioncontrollerlefft) 1000.0)) :`ObjectTypes` (`|MakeArray` "ObjectTypeQuery4" :!type "EObjectTypeQuery Enum") :`DrawDebugType` "ForDuration"))
  (if _returnvalue_2
    (bind (_bblockinghit _binitialoverlap _time _distance _location _impactpoint _normal _impactnormal _physmat _hitactor _hitcomponent) (`GameplayStatics.BreakHitResult` _outhit))
    (set `self.Hit Component` _hitcomponent)
    (if (`SceneComponent.IsAnySimulatingPhysics` _hit_component)
      (bind _output_get (set `self.Picked Up Actor` _hitactor))
      (`PrimitiveComponent.SetSimulatePhysics` _hit_component false)
      (`self.K2_AttachToComponent` _output_get (`self.MotionControllerLefft`) "None" "SnapToTarget" "SnapToTarget" "KeepWorld" true)
      (set `self.Is Holding Object` true))))

(event `DropObject`
  (bind _picked_up_actor (`self.Picked Up Actor`))
  (bind _hit_component (`self.Hit Component`))
  ;[0.6037 0.6046 0.9635] Drop Object
  (`/Engine/EditorBlueprintResources/StandardMacros.IsValid` _picked_up_actor
    (:`Is Valid`
      (`self.K2_DetachFromActor` _picked_up_actor "KeepWorld" "KeepWorld" "KeepWorld")
      (`/Engine/EditorBlueprintResources/StandardMacros.IsValid` _hit_component
        (:`Is Valid`
          (`PrimitiveComponent.SetSimulatePhysics` _hit_component true)
          (set `self.Is Holding Object` false)
          (set `self.Hit Component` null)
          (set `self.Picked Up Actor` null))))))

(fn `UserConstructionScript`)